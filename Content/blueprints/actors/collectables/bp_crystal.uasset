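; Crystal collectable that destroys itself after any actor overlaps it.
; Overlap starts three timelines, including Miganie (blinking), with only Finished outputs wired: they zero the point light's IES brightness or actor scale, and whichever finishes first destroys the actor.
; A Polish-named move-toward-player function runs first for the player pawn, but its zero lerp alpha leaves the crystal in place.
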(event `self.ReceiveActorBeginOverlap`
  (params (OtherActor :type "Actor Object Reference"))
  (`self.przesuwanie obiektu w stronę gracza` OtherActor)
  (`|ExecutionSequence`
    (:`then_0`
      (`Timeline|miganie`
        (:`Finished`
          (`LightComponent.SetIESBrightnessScale` (`self.PointLight`) 0.0))))
    (:`then_1`
      (`Timeline|Timeline_0`
        (:`Finished`
          _)))
    (:`then_2`
      (`Timeline|Timeline_2`
        (:`Finished`
          (`self.SetActorScale3D` (0.0 0.0 0.0))))))
  (`self.K2_DestroyActor`))

(fn `przesuwanie obiektu w stronę gracza`
  (params (A :type "Object Object Reference"))
  (if (== A (`GameplayStatics.GetPlayerPawn` 0))
    (`self.K2_SetActorLocation` self (`KismetMathLibrary.VLerp` (`self.K2_GetActorLocation` self) (`self.K2_GetActorLocation` (`GameplayStatics.GetPlayerPawn` 0))) false false)))

(fn `UserConstructionScript`)